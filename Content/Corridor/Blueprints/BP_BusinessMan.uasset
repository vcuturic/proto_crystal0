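; BP_BusinessMan is an AI-moved businessman pawn that carries a briefcase along a route of destination actors.
; On BeginPlay it snaps the referenced briefcase to a hand socket on its mesh and stores that socket's component-space transform.
; It chains AI Move To calls through the Destinations array on each success, destroying itself after the last.
; A separate Enlarge event doubles the actor's scale.
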(event Custom|Enlarge
  (Transformation|SetActorScale3D "2.000000,2.000000,2.000000"))

(event EventBeginPlay
  (bind _self self)
  (bind _destinations (Variables|Default|GetDestinations))
  (bind _mesh (Variables|Character|GetMesh))
  (Transformation|AttachComponentToComponent (Variables|Default|GetBriefcaseRef) _mesh "BriefcaseSocket" "SnapToTarget" "SnapToTarget" "KeepWorld" false)
  (Variables|Default|SetHandTransform (Transformation|GetSocketTransform _mesh "BriefcaseSocket" "RTS_Component"))
  (AI|AIMoveTo _self "0, 0, 0" (Utilities|Array|Get(acopy) _destinations (Variables|Default|GetTarget%20Point)) 5.0 false :!label _label
    (:OnSuccess
      (if (== (+ (Variables|Default|GetTarget%20Point) 1) (Utilities|Array|Length _destinations))
        (Variables|Default|SetTarget%20Point 0)
        (Actor|DestroyActor _self)
        (else
          (Variables|Default|SetTarget%20Point (+ (Variables|Default|GetTarget%20Point) 1))
          (goto _label))))))

(fn ConstructionScript)